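; Master gun Blueprint that fires Rin projectiles in Single, Burst or Auto mode.
; StartFire spawns a scaled-down projectile at the Muzzle socket, aimed by MuzzleRotator, either directly or on Fire events from the Burst and Auto timelines.
; StopFire rewinds and stops only the Auto timeline, so a started burst is not interrupted.
; SwitchFireMode cycles through the three modes in order.
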(event Custom|StartFire
  ;[1 1 1] Start Fire
  (switch Utilities|FlowControl|Switch|SwitchonFireMode (Variables|Default|GetFireMode)
    (:NewEnumerator0
      _)
    (:NewEnumerator1
      (Timeline|Burst PlayFromStart
        (:Fire
          _)))
    (:NewEnumerator2
      (Timeline|Auto Play
        (:Fire
          _))))
  (Game|SpawnActorfromClass "/Game/Rin/BluePrints/Projectile/Rin_Projectile_Master_BP.Rin_Projectile_Master_BP_C" (Math|Transform|MakeTransform (.Location (Math|Transform|BreakTransform (Transformation|GetSocketTransform (Variables|Default|GetSkeletalMesh) "Muzzle" "RTS_World"))) (Variables|Default|GetMuzzleRotator) "0.100000,0.100000,0.100000") "AlwaysSpawn" 0 0))

(event Custom|StopFire
  ;[1 1 1] Start Fire
  (Utilities|FlowControl|Sequence
    (:then_0
      (Timeline|Auto SetNewTime
        (:Fire
          (Game|SpawnActorfromClass "/Game/Rin/BluePrints/Projectile/Rin_Projectile_Master_BP.Rin_Projectile_Master_BP_C" (Math|Transform|MakeTransform (.Location (Math|Transform|BreakTransform (Transformation|GetSocketTransform (Variables|Default|GetSkeletalMesh) "Muzzle" "RTS_World"))) (Variables|Default|GetMuzzleRotator) "0.100000,0.100000,0.100000") "AlwaysSpawn" 0 0))))
    (:then_1
      (Timeline|Auto Stop))))

(fn ConstructionScript)

(fn SwitchFireMode
  (switch Utilities|FlowControl|Switch|SwitchonFireMode (Variables|Default|GetFireMode)
    (:NewEnumerator0
      (Variables|Default|SetFireMode "NewEnumerator1"))
    (:NewEnumerator1
      (Variables|Default|SetFireMode "NewEnumerator2"))
    (:NewEnumerator2
      (Variables|Default|SetFireMode "NewEnumerator0"))))